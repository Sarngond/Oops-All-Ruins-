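; Multiplayer GameState that tracks the player list, the qualified players and the number of players needed to qualify.
; Events copy PlayerArray into AllPlayerStates and store the qualification values passed to them.
; RepNotify functions find every player list or gameplay HUD widget by class and refresh it when the matching player data changes.
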(event Custom|Update_PlayerList
  (Variables|Default|SetAll%20Player%20States (Variables|Default|GetPlayerArray)))

(event Custom|Update_QualifiedPlayers
  (params (Qualified%20Players :type Integer))
  (Variables|Default|SetQualified%20Players Qualified%20Players))

(event Custom|Set_NumberToQualify
  (params (NumberToQualify :type Integer))
  (Variables|Default|SetNumberToQualify NumberToQualify))

(fn ConstructionScript)

(fn OnRepAllPlayerStates
  (bind _foundwidgets (Widget|GetAllWidgetsOfClass "/Game/Widgets/WB_PlayerList.WB_PlayerList_C" false))
  (for _array_element _foundwidgets
    (Default|UpdateWidget _array_element)))

(fn OnRepQualifiedPlayers
  (bind _foundwidgets (Widget|GetAllWidgetsOfClass "/Game/Widgets/WB_GameplayHUD.WB_GameplayHUD_C" false))
  (for _array_element _foundwidgets
    (Default|UpdatePlayersQualified _array_element)))

(fn OnRepAllPlayers)
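; Multiplayer player controller that handles spawning, respawning and teleporting of its player.
; On BeginPlay the local controller picks a random PlayerStart and passes its transform to a spawn event, which waits out a delay then calls SpawnPlayer on BP_GM_BasicSetup.
; Helpers clear widgets, store a checkpoint transform and teleport a character.
; Spectator, qualification, end-check and leave-session events are empty, their logic left disconnected.
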(event Custom|Leave%20Session)

(event Custom|Check%20if%20End
  (params (Condition :type Boolean)))

(event Custom|Set%20Qualified
  (params (qualified :type Boolean)))

(event Custom|Clear%20Screen
  ;[0.15 0.15 0.15 0.5] Clear Widgets
  (Viewport|RemoveAllWidgets))

(event Custom|SR_SpawnPlayer
  (params (Respawn%20Delay :type Float%20%28double-precision%29) (Checkpoint%20Transform :type Transform))
  ;[0.15 0.15 0.15 0.5] Spawn Player
  (bind _asbp_gm_basic_setup (Utilities|Casting|CastToBP_GM_BasicSetup (Game|GetGameMode)))
  (Utilities|FlowControl|Delay Respawn%20Delay)
  (Default|SpawnPlayer _asbp_gm_basic_setup self Checkpoint%20Transform))

(event Custom|TeleportPlayer
  (params (Player%20Character :type Actor%20Object%20Reference) (TeleportLocation :type Vector))
  (Transformation|SetActorLocation Player%20Character TeleportLocation false true)
  (Development|PrintString "Player Teleported"))

(event Custom|SetPlayerAsSpectator)

(event EventBeginPlay
  (if (Pawn|IsLocalPlayerController)
    (bind _outactors (Actor|GetAllActorsOfClass "/Script/Engine.PlayerStart"))
    (bind _output_get (Variables|Default|SetCheckpointTransform (Transformation|GetActorTransform (Utilities|Array|Get(acopy) _outactors (Math|Random|RandomIntegerinRange 0 (- (Utilities|Array|Length _outactors) 1))))))
    (CallFunction|SRSpawnPlayer 0.0 _output_get)))

(fn ConstructionScript)

(fn SetPlayerCheckpoint
  (params (Checkpoint%20Location :type Transform))
  (Variables|Default|SetCheckpointTransform Checkpoint%20Location))
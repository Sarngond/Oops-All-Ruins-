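; Multiplayer game mode that tracks connected player controllers and active players, and provides spawning and map travel.
; Login, controller swap and logout events maintain the controller list, while a separate event adds active players and prints a debug message.
; SpawnPlayer replaces a controller's pawn with a new BP_SkellyMultiplayer at a given checkpoint transform.
; Helpers return a random PlayerStart transform, and TravelTo changes level through a servertravel console command.
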(event Custom|Travel%20To
  (params (LevelName :type String))
  (Development|ExecuteConsoleCommand (Utilities|String|Append "servertravel " LevelName) 0))

(event Custom|AddPlayersToActive
  (params (Player :type Character%20Object%20Reference%20%28by%20ref%29))
  (Utilities|Array|Add (Variables|Default|GetPlayersActive) Player)
  (Development|PrintString (Utilities|String|Append (Utilities|String|ToString(Object) Player) "Added to list")))

(event Custom|CustomEvent)

(event EventPostLogin
  (params (NewPlayer :type Player%20Controller%20Object%20Reference))
  ;[1 1 1] Player Connection / Disconnection
  ;;[1 1 1] Event for when a player conncets
  (Utilities|Array|Add (Variables|Default|GetAll%20Player%20Controllers) NewPlayer))

(event EventOnSwapPlayerControllers
  (params (OldPC :type Player%20Controller%20Object%20Reference) (NewPC :type Player%20Controller%20Object%20Reference))
  ;[1 1 1] Player Connection / Disconnection
  ;;[1 1 1] Event for when a player conncets
  (Utilities|Array|Add (Variables|Default|GetAll%20Player%20Controllers) NewPC))

(event EventOnLogout
  (params (ExitingController :type Controller%20Object%20Reference))
  ;[1 1 1] Player Connection / Disconnection
  ;;[1 1 1] Event for when a player disconnects
  (bind _asbp_pc_basic_setup (Utilities|Casting|CastToBP_PC_BasicSetup ExitingController))
  (Utilities|Array|RemoveItem (Variables|Default|GetAll%20Player%20Controllers) _asbp_pc_basic_setup))

(fn ConstructionScript)

(fn FindRandomPlayerStart
  (bind _outactors (Actor|GetAllActorsOfClass "/Script/Engine.PlayerStart"))
  (return (Transformation|GetActorTransform (Utilities|Array|Get(acopy) _outactors (Math|Random|RandomIntegerinRange 0 (- (Utilities|Array|Length _outactors) 1))))))

(fn SpawnPlayer
  (params (Target :type Controller%20Object%20Reference) (Checkpoint%20Transform :type Transform))
  (bind _returnvalue (Pawn|GetControlledPawn Target))
  (Utilities|IsValid _returnvalue
    (:Is%20Valid
      (Actor|DestroyActor _returnvalue))
    (:Is%20Not%20Valid
      _))
  (bind _returnvalue_2 (Game|SpawnActorfromClass "/Game/Multiplayer/BP_SkellyMultiplayer.BP_SkellyMultiplayer_C" Checkpoint%20Transform "Undefined" "MultiplyWithRoot" 0 0))
  (Pawn|Possess Target _returnvalue_2))

(fn GetRandomPlayerStart
  (return (CallFunction|FindRandomPlayerStart)))
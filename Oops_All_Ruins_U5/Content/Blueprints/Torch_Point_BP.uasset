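; Torch point light Blueprint with graph logic for flickering and vertical movement, none of which is connected to run.
; BeginPlay and the construction script are empty.
; The orphaned flicker chain waits a random delay, then scales a timeline curve by random noise to set light intensity.
; Separate orphaned chains store the light's start position, play a second timeline and offset the light's height from it.
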(event EventBeginPlay)

(fn ConstructionScript)
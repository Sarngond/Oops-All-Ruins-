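; Torch actor Blueprint with a SpotLight and unfinished or disabled logic for a flickering flame effect.
; The flicker chain waits a random delay, then drives light intensity from the Flickering timeline scaled by a random multiplier.
; Separate chains store the light's start location and offset its height by Timeline_0's value.
; None of these chains connect to an event, and BeginPlay and the construction script are empty.
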(event EventBeginPlay)

(fn ConstructionScript)
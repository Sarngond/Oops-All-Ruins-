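; Torch Blueprint, a less intense variant going by its name, with a spot light and unconnected logic for animating it.
; BeginPlay and the construction script are empty, so none of the graph logic runs.
; The orphaned nodes hold a randomly delayed timeline intensity flicker with random scaling, plus fragments for moving the light vertically from its initial position with a second timeline.
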(event EventBeginPlay)

(fn ConstructionScript)
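; Torch point light actor that flickers, named as a less intense variant.
; On BeginPlay it waits a short random delay, then plays the Flickering timeline.
; Each timeline update sets the PointLight intensity from the scaled curve value times a fresh random multiplier, adding jitter.
; A Move timeline for offsetting the light vertically from its initial position is present but never runs.
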(event EventBeginPlay
  (Utilities|FlowControl|Delay (Math|Random|RandomFloatinRange 0.0 0.8))
  (bind _intensity (Timeline|flickering Play)
    (:Update
      (Rendering|Components|Light|SetIntensity (Variables|Default|GetPointLight) (* (* _intensity 2e+03) (Math|Random|RandomFloatinRange 1.0 1.5))))))

(fn ConstructionScript)
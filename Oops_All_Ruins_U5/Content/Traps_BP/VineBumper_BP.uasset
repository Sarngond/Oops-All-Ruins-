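; Vine bumper trap that bounces small boulders away and pulses its mesh when hit.
; Capsule overlap with a SmallBoulder_BP applies a velocity-change impulse: combined bumper and boulder velocity, reversed horizontally and scaled by Bouncyness, plus a fixed upward kick.
; A shared timeline offsets the mesh's initial X and Y scale, replaying on boulder hits or third-person character overlaps, which receive no impulse.
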(event OnComponentBeginOverlap(Capsule)
  (params (OverlappedComponent :type Primitive%20Component%20Object%20Reference) (OtherActor :type Actor%20Object%20Reference) (OtherComp :type Primitive%20Component%20Object%20Reference) (OtherBodyIndex :type Integer) (bFromSweep :type Boolean) (SweepResult :type Hit%20Result%20Structure%20%28by%20ref%29))
  (bind _initscale (Variables|Default|GetInitScale))
  (bind _assmall_boulder_bp (Utilities|Casting|CastToSmallBoulder_BP OtherActor))
  (Physics|AddImpulse (Variables|/Game/Traps_BP/SmallBoulder_BP.SmallBoulder_BP_C|GetBoulder _assmall_boulder_bp) (Math|Vector|MakeVector (.x (* (+ (Transformation|GetVelocity) (Transformation|GetVelocity _assmall_boulder_bp)) (* (Variables|Default|GetBouncyness) "-1.000000,-1.000000,0.000000"))) (.y (* (+ (Transformation|GetVelocity) (Transformation|GetVelocity _assmall_boulder_bp)) (* (Variables|Default|GetBouncyness) "-1.000000,-1.000000,0.000000"))) 3e+02) "None" true)
  (bind _newtrack_0 (Timeline|Timeline_0 PlayFromStart)
    (:Update
      (Transformation|SetRelativeScale3D (Variables|Default|GetVine_Bumber_LowPoly_Geo) (Math|Vector|MakeVector (+ (.x _initscale) _newtrack_0) (+ (.y _initscale) _newtrack_0) (.z _initscale))))))

(event Collision|EventActorBeginOverlap
  (params (OtherActor :type Actor%20Object%20Reference))
  (bind _initscale (Variables|Default|GetInitScale))
  (Utilities|Casting|CastToBP_ThirdPersonCharacter OtherActor)
  (bind _newtrack_0 (Timeline|Timeline_0 PlayFromStart)
    (:Update
      (Transformation|SetRelativeScale3D (Variables|Default|GetVine_Bumber_LowPoly_Geo) (Math|Vector|MakeVector (+ (.x _initscale) _newtrack_0) (+ (.y _initscale) _newtrack_0) (.z _initscale))))))

(event EventTick
  (params (DeltaSeconds :type Float%20%28single-precision%29)))

(event EventBeginPlay
  (Variables|Default|SetInitScale (Variables|/Script/Engine.SceneComponent|GetRelativeScale3D (Variables|Default|GetVine_Bumber_LowPoly_Geo))))

(fn ConstructionScript)
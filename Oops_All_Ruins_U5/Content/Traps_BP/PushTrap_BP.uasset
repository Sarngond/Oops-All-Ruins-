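; PushTrap is a trap actor that slides its mesh back and forth or outward along world Y and launches skeleton player characters that overlap it.
; On BeginPlay it stores the mesh position, waits a random delay, then drives the Y offset with a timeline that replays after a short random pause.
; Overlap applies a fixed world-space launch toward negative Y and upward, independent of the timeline's state.
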(event Custom|Start%20Movement
  (Variables|Default|SetInitPos (Transformation|GetWorldLocation (Variables|Default|GetStaticMesh)))
  (Utilities|FlowControl|Delay (Math|Random|RandomFloatinRange 0.0 5.0))
  (bind _push (Timeline|Timeline_0 Play)
    (:Update
      (Transformation|SetWorldLocation (Variables|Default|GetStaticMesh) (Math|Vector|MakeVector (.x (Variables|Default|GetInitPos)) (+ _push (.y (Variables|Default|GetInitPos))) (.z (Variables|Default|GetInitPos))) false false))
    (:Finished
      (Utilities|FlowControl|Delay (Math|Random|RandomFloatinRange 0.0 1.0))
      (Timeline|Timeline_0 PlayFromStart))))

(event EventBeginPlay
  (CallFunction|StartMovement))

(event Collision|EventActorBeginOverlap
  (params (OtherActor :type Actor%20Object%20Reference))
  (bind _asbp_skelly_multiplayer (Utilities|Casting|CastToBP_SkellyMultiplayer OtherActor))
  (Character|LaunchCharacter _asbp_skelly_multiplayer "0.000000,-100.000000,100.000000" false true))

(event EventTick
  (params (DeltaSeconds :type Float%20%28single-precision%29)))

(fn ConstructionScript)
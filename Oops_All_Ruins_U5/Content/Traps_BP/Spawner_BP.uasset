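; Trap spawner actor that endlessly spawns a configurable Object class at the location of its Spawn component.
; BeginPlay chains through events named for server and client into the spawn loop, which captures the location once.
; A random initial delay staggers the first spawn, then a looping Delay repeats it at SpawnRate plus slight random jitter.
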(event Custom|Spawn%20Object%20on%20client
  (Variables|Default|SetspawnLocation (Transformation|GetWorldLocation (Variables|Default|GetSpawn)))
  (Utilities|FlowControl|Delay (Math|Random|RandomFloatinRange 0.0 2.0))
  (Game|SpawnActorfromClass (Variables|Default|GetObject) (Math|Transform|MakeTransform (Variables|Default|GetspawnLocation) "0, 0, 0" "1.000000,1.000000,1.000000") "Undefined" 0 0 :!label _label)
  (Utilities|FlowControl|Delay (+ (Variables|Default|GetspawnRate) (Math|Random|RandomFloatinRange 0.0 0.3)))
  (goto _label))

(event Custom|Spawn%20Object%20on%20server
  (CallFunction|SpawnObjectonClient))

(event EventBeginPlay
  (CallFunction|SpawnObjectonServer))

(event Collision|EventActorBeginOverlap
  (params (OtherActor :type Actor%20Object%20Reference)))

(fn ConstructionScript)